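; Wind indicator arrow that rolls to show the current wind direction and strength from the game mode.
; Tick watches for WindSpeed changes, then picks a target roll from WindDirection: zero for case 0, otherwise left or right scaled by speed.
; Delay-driven loops ease the arrow root there with RInterpTo, using MovingLeft and MovingRight flags to cancel opposing turns.
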(event EventBeginPlay)

(event Collision|EventActorBeginOverlap
  (params (OtherActor :type Actor%20Object%20Reference)))

(event EventTick
  (params (DeltaSeconds :type Float%20%28single-precision%29))
  (bind _gamemoderef (Variables|Default|GetGameModeRef))
  (bind _arrowroot (Variables|Default|GetArrowRoot))
  (bind _windspeed (Variables|/Game/HandheldARBP/Blueprints/GameFramework/BP_ARGameMode.BP_ARGameMode_C|GetWindSpeed _gamemoderef))
  (bind _relativerotation (Variables|/Script/Engine.SceneComponent|GetRelativeRotation _arrowroot))
  (Variables|Default|SetDelta DeltaSeconds)
  (if (not (== (Variables|Default|GetZRotOld) _windspeed))
    (Variables|Default|SetZRotOld _windspeed)
    (switch int (Variables|/Game/HandheldARBP/Blueprints/GameFramework/BP_ARGameMode.BP_ARGameMode_C|GetWindDirection _gamemoderef)
      (:0
        ;[0 0 0] Lerp Arrow to new direction
        (Variables|Default|SetMoving%20right false)
        (Variables|Default|SetMoving%20Left false)
        (if (not (Math|Rotator|Equal(Rotator) _relativerotation "0, 0, 0" 0.01)) :!label _label
          (Transformation|SetRelativeRotation (Variables|Default|GetArrowRoot) (Math|Interpolation|RInterpTo _relativerotation "0, 0, 0" (Variables|Default|GetDelta) 1.0) false false)
          (if (not (and (Variables|Default|GetMoving%20right) (Variables|Default|GetMoving%20Left)))
            (Utilities|FlowControl|Delay 0.01)
            (goto _label))))
      (:1
        (Variables|Default|SetMoving%20right true)
        (Variables|Default|SetMoving%20Left false)
        (if (not (Math|Rotator|Equal(Rotator) _relativerotation (Math|Rotator|MakeRotator (* (* (/ (Math|Float|Absolute(Float) (Variables|Default|GetZRotOld)) 4.0) 9e+01) -1.0) 0.0 0.0) 0.01)) :!label _label_2
          (Transformation|SetRelativeRotation (Variables|Default|GetArrowRoot) (Math|Interpolation|RInterpTo _relativerotation (Math|Rotator|MakeRotator (* (* (/ (Math|Float|Absolute(Float) (Variables|Default|GetZRotOld)) 4.0) 9e+01) -1.0) 0.0 0.0) (Variables|Default|GetDelta) 1.0) false false)
          (if (Variables|Default|GetMoving%20right)
            (Utilities|FlowControl|Delay 0.01)
            (goto _label_2))))
      (:2
        (Variables|Default|SetMoving%20Left true)
        (Variables|Default|SetMoving%20right false)
        (if (not (Math|Rotator|Equal(Rotator) _relativerotation (Math|Rotator|MakeRotator (* (/ (Math|Float|Absolute(Float) (Variables|Default|GetZRotOld)) 4.0) 9e+01) 0.0 0.0) 0.01)) :!label _label_3
          (Transformation|SetRelativeRotation (Variables|Default|GetArrowRoot) (Math|Interpolation|RInterpTo _relativerotation (Math|Rotator|MakeRotator (* (/ (Math|Float|Absolute(Float) (Variables|Default|GetZRotOld)) 4.0) 9e+01) 0.0 0.0) (Variables|Default|GetDelta) 1.0) false false)
          (if (Variables|Default|GetMoving%20Left)
            (Utilities|FlowControl|Delay 0.01)
            (goto _label_3)))))))

(fn ConstructionScript)